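; Lamp post hazard whose spotlight switches on and off on a timer and kills the player caught in it while lit.
; A looping timer drives a FlipFlop that toggles the LightOn flag, spotlight visibility, trigger box collision and lamp glass material together.
; When the box begins overlapping the ThirdPersonCharacter's capsule with the light on, it calls KillPlayer on that character.
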(event `self.ReceiveBeginPlay`
  (bind _returnvalue (`KismetSystemLibrary.K2_SetTimerDelegate` (delegate `SetKillBool`) 3.0 true))
  (`KismetSystemLibrary.PrintString` (`KismetStringLibrary.Conv_DoubleToString` (`KismetSystemLibrary.K2_GetTimerElapsedTimeHandle` _returnvalue)) true true (struct :`G` 0.66 :`B` 1.0 :`A` 1.0) 0.01))

(event `SetKillBool`
  (bind _box (`self.Box`))
  (bind _lamppost (`self.LampPost`))
  (`/Engine/EditorBlueprintResources/StandardMacros.FlipFlop`
    (:`A`
      (set `self.LightOn` true)
      (`SceneComponent.SetVisibility` (`self.SpotLight`) true false)
      (`PrimitiveComponent.SetCollisionEnabled` _box "QueryOnly")
      (`PrimitiveComponent.SetMaterial` _lamppost 2 "/Game/Assets/LampPost/Glass.Glass"))
    (:`B`
      (set `self.LightOn` false)
      (`SceneComponent.SetVisibility` (`self.SpotLight`) false false)
      (`PrimitiveComponent.SetCollisionEnabled` _box "NoCollision")
      (`PrimitiveComponent.SetMaterial` _lamppost 2 "/Game/Assets/LampPost/Glass_Inst.Glass_Inst"))))

(event `self.Box.OnComponentBeginOverlap`
  (params (OverlappedComponent :type "PrimitiveComponent Object Reference") (OtherActor :type "Actor Object Reference") (OtherComp :type "PrimitiveComponent Object Reference") (OtherBodyIndex :type Integer) (bFromSweep :type Boolean) (SweepResult :type "HitResult Structure (by ref)"))
  (bind _asthird_person_character (cast `/Game/ThirdPersonBP/ThirdPersonCharacter` OtherActor))
  (if (and (`self.LightOn`) (== OtherComp (`Character.CapsuleComponent` _asthird_person_character)))
    (`/Game/ThirdPersonBP/ThirdPersonCharacter.KillPlayer` _asthird_person_character)))

(fn `UserConstructionScript`)