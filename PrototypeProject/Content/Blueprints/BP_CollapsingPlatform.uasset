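; BP_CollapsingPlatform is a platform that falls away and destroys itself when a ThirdPersonCharacter steps on it.
; The Box overlap checks for the character's capsule, plays a wood-break sound at the world origin and starts the UpdateFallingPlatform timeline from the beginning.
; Each timeline update subtracts the FallingDuration track value from the mesh's current world Z, so the drop accumulates per update, and the actor is destroyed when the timeline finishes.
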(event `self.Box.OnComponentBeginOverlap`
  (params (OverlappedComponent :type "PrimitiveComponent Object Reference") (OtherActor :type "Actor Object Reference") (OtherComp :type "PrimitiveComponent Object Reference") (OtherBodyIndex :type Integer) (bFromSweep :type Boolean) (SweepResult :type "HitResult Structure (by ref)"))
  (bind _mesh (`self.Mesh`))
  (bind (_returnvalue_x _returnvalue_y _returnvalue_z) (`KismetMathLibrary.BreakVector` (`SceneComponent.K2_GetComponentLocation` _mesh)))
  (bind _asthird_person_character (cast `/Game/ThirdPersonBP/ThirdPersonCharacter` OtherActor))
  (if (== OtherComp (`Character.CapsuleComponent` _asthird_person_character))
    (`GameplayStatics.PlaySoundAtLocation` "/Game/Audio/wood_break_Cue.wood_break_Cue" (0.0 0.0 0.0) (struct) 1.0 1.0 0.0 null null null)
    (bind (_direction _fallingduration) (`Timeline|UpdateFallingPlatform` :!via `PlayFromStart`)
      (:`Update`
        (`SceneComponent.K2_SetWorldLocation` _mesh (`KismetMathLibrary.MakeVector` _returnvalue_x _returnvalue_y (- _returnvalue_z _fallingduration)) false false))
      (:`Finished`
        (`self.K2_DestroyActor`)))))

(fn `UserConstructionScript`)