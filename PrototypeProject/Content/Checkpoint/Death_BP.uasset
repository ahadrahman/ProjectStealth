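; Death volume actor that respawns the player at the last saved checkpoint when its DeathTrigger is overlapped.
; The overlap, which does not check the overlapping actor, disables the ThirdPersonCharacter's input and waits briefly.
; If the "check" save slot exists, it moves the character to the saved SaveTut location and re-enables input.
; Without a save, it opens a level by name instead.
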(event `self.Death Trigger.OnComponentBeginOverlap`
  (params (OverlappedComponent :type "PrimitiveComponent Object Reference") (OtherActor :type "Actor Object Reference") (OtherComp :type "PrimitiveComponent Object Reference") (OtherBodyIndex :type Integer) (bFromSweep :type Boolean) (SweepResult :type "HitResult Structure (by ref)"))
  (bind _asthird_person_character (cast `/Game/ThirdPersonBP/ThirdPersonCharacter` (`GameplayStatics.GetPlayerCharacter` 0)))
  (`self.DisableInput` _asthird_person_character (`GameplayStatics.GetPlayerController` 0))
  (`KismetSystemLibrary.Delay` 0.02)
  (bind _returnvalue (`GameplayStatics.DoesSaveGameExist` "check"))
  (if _returnvalue
    (bind _returnvalue_2 (`GameplayStatics.LoadGameFromSlot` "check"))
    (bind _assave_tut (cast `/Game/Checkpoint/SaveTut` _returnvalue_2))
    (bind _asthird_person_character_2 (cast `/Game/ThirdPersonBP/ThirdPersonCharacter` (`GameplayStatics.GetPlayerCharacter` 0)))
    (`self.K2_SetActorLocation` _asthird_person_character_2 (`/Game/Checkpoint/SaveTut.PlayerLoc_s` _assave_tut) false false)
    (`self.EnableInput` _asthird_person_character_2 (`GameplayStatics.GetPlayerController` 0))
    (else
      (`GameplayStatics.OpenLevel` (`self.Level`)))))

(fn `UserConstructionScript`)