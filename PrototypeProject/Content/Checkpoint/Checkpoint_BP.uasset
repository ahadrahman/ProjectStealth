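; Checkpoint actor that saves the player's location when the third-person character's capsule overlaps its trigger.
; With its Load flag on, it writes location and a load flag to the "check" SaveTut slot, creating the save if absent, then turns its spotlight yellow after a short delay.
; With the flag off, it instead clears the saved load flag, acting as a checkpoint reset.
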(event `self.Trigger.OnComponentBeginOverlap`
  (params (OverlappedComponent :type "PrimitiveComponent Object Reference") (OtherActor :type "Actor Object Reference") (OtherComp :type "PrimitiveComponent Object Reference") (OtherBodyIndex :type Integer) (bFromSweep :type Boolean) (SweepResult :type "HitResult Structure (by ref)"))
  (bind _playerloc (`self.PlayerLoc`))
  (bind _asthird_person_character (cast `/Game/ThirdPersonBP/ThirdPersonCharacter` OtherActor))
  (if (== OtherComp (`Character.CapsuleComponent` _asthird_person_character))
    (if (`self.Load?`)
      (`|ExecutionSequence`
        (:`then_0`
          ;[1 1 1] Sets variable PlayerLoc to our player's current location
          (bind _asthird_person_character_2 (cast `/Game/ThirdPersonBP/ThirdPersonCharacter` (`GameplayStatics.GetPlayerCharacter` 0)))
          (set `self.PlayerLoc` (`self.K2_GetActorLocation` _asthird_person_character_2))
          (`KismetSystemLibrary.PrintString` "Checkpoint reached!"))
        (:`then_1`
          (bind _returnvalue (`GameplayStatics.DoesSaveGameExist` "check"))
          (if _returnvalue
            (bind _returnvalue_2 (`GameplayStatics.LoadGameFromSlot` "check"))
            (bind _assave_tut (cast `/Game/Checkpoint/SaveTut` _returnvalue_2))
            (set `/Game/Checkpoint/SaveTut.PlayerLoc_s` _playerloc _assave_tut)
            (set `/Game/Checkpoint/SaveTut.Load?` true _assave_tut)
            (`GameplayStatics.SaveGameToSlot` _assave_tut "check")
            (else
              ;[1 1 1] Saves that variable to "SaveTut" if there's no save game object
              (bind _returnvalue_3 (`GameplayStatics.CreateSaveGameObject` "/Game/Checkpoint/SaveTut.SaveTut_C"))
              (set `/Game/Checkpoint/SaveTut.PlayerLoc_s` _playerloc _returnvalue_3)
              (set `/Game/Checkpoint/SaveTut.Load?` true _returnvalue_3)
              (`GameplayStatics.SaveGameToSlot` _returnvalue_3 "check")))
          (`KismetSystemLibrary.Delay` 0.4)
          (`LightComponent.SetLightColor` (`self.SpotLight`) (struct :`R` 1.0 :`G` 0.913283 :`A` 1.0) true)))
      (else
        (bind _returnvalue_4 (`GameplayStatics.LoadGameFromSlot` "check"))
        (bind _assave_tut_2 (cast `/Game/Checkpoint/SaveTut` _returnvalue_4))
        (set `/Game/Checkpoint/SaveTut.Load?` false _assave_tut_2)
        (`GameplayStatics.SaveGameToSlot` _assave_tut_2 "check")
        (`KismetSystemLibrary.PrintString` "Checkpoint cleared.")))))

(fn `UserConstructionScript`)